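; Demi-boss character Blueprint that chases the player.
; After a short delay on BeginPlay, it starts a self-restarting seek loop that reissues AI MoveTo toward the player character twice a second.
; A looping timer also runs PlayerDistance every second to compare the boss-to-player distance against a threshold, but both branches only print the same placeholder string.
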(event Custom|SeekPlayer
  ;[1 1 1] Seek Player Loop
  (AI|AIMoveTo self "0, 0, 0" (Game|GetPlayerCharacter 0) 2e+02 false
    (:then
      _)
    (:OnSuccess
      _)
    (:OnFail
      _))
  (Utilities|FlowControl|Delay 0.5)
  (CallFunction|SeekPlayer))

(event Custom|DistancePlayer
  (Utilities|Time|SetTimerbyFunctionName 0 "PlayerDistance" 1.0 true))

(event EventBeginPlay
  ;[1 1 1] Initialize Boss
  (Utilities|FlowControl|Delay 0.2)
  (CallFunction|SeekPlayer)
  (CallFunction|DistancePlayer))

(fn ConstructionScript)

(fn PlayerDistance
  (bind _output_get (Variables|Default|SetDistance (Math|Vector|VectorLength (- (Transformation|GetActorLocation) (Transformation|GetActorLocation (Game|GetPlayerCharacter 0))))))
  (if (>= _output_get 6e+02)
    (Development|PrintString "Hello" true true "(R=1.000000,G=0.071750,B=0.051854,A=1.000000)")
    (else
      (Development|PrintString "Hello"))))